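; BP_NPC_Master is the base interactable NPC that runs dialogue with the player.
; Construction loads its dialogue from NPC_Dialogue by NPCID.
; OnInteract registers itself as dialogue partner, switches and locks the camera, reuses or creates the player's WB_DialogueBox, and enables UI-only input.
; CreateDialogue shows the current line, or closes the box when the conversation ends, restoring camera and game input and resetting the line index.
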(event Custom|CloseDialogueBox
  (bind _playercontrollerref (Variables|References|GetPlayerControllerRef))
  ;[1 1 1] CloseDialogue Box
  (Widget|SetVisibility (Variables|/Game/Player/Blueprints/BP_Player_Character.BP_Player_Character_C|GetDialogueRef (Variables|References|GetPlayerRef)) "Hidden")
  (Default|SwitchCameraViewTarget (Variables|References|GetPlayerControllerRef) false (Variables|Default|GetCameraBlendTime))
  (Utilities|FlowControl|Delay (Variables|Default|GetCameraBlendTime))
  (Input|SetInputModeGameOnly _playercontrollerref false)
  (Variables|/Script/Engine.PlayerController|SetbShowMouseCursor _playercontrollerref false)
  (Default|LockCamera (Variables|References|GetPlayerControllerRef) false))

(event EventOnInteract
  (params (PlayerRef :type BP%20Player%20Character%20Object%20Reference) (ControllerRef :type BP%20Player%20Controller%20Object%20Reference))
  (Utilities|FlowControl|Sequence
    (:then_0
      ;[1 1 1] Set References to player
      (Utilities|IsValid (Variables|References|GetPlayerRef)
        (:Is%20Not%20Valid
          (Variables|References|SetPlayerRef PlayerRef))))
    (:then_1
      (Utilities|IsValid (Variables|References|GetPlayerControllerRef)
        (:Is%20Not%20Valid
          (Variables|References|SetPlayerControllerRef ControllerRef))))
    (:then_2
      ;[1 1 1] Set Dialogue Member
      (Variables|/Game/Player/Blueprints/BP_Player_Character.BP_Player_Character_C|SetDialoguePartner (Variables|References|GetPlayerRef) self))
    (:then_3
      (Default|SwitchCameraViewTarget (Variables|References|GetPlayerControllerRef) true (Variables|Default|GetCameraBlendTime))
      (Default|LockCamera (Variables|References|GetPlayerControllerRef) true)
      (Utilities|FlowControl|Delay 0.2)
      ;[1 1 1] Create Dialogue Widget
      (Utilities|IsValid (Variables|/Game/Player/Blueprints/BP_Player_Character.BP_Player_Character_C|GetDialogueRef (Variables|References|GetPlayerRef))
        (:Is%20Valid
          (Default|GetConversationPartner (Variables|/Game/Player/Blueprints/BP_Player_Character.BP_Player_Character_C|GetDialogueRef (Variables|References|GetPlayerRef)) "NewEnumerator0" (Variables|References|GetPlayerRef))
          (Default|InitialiseDialogue (Variables|/Game/Player/Blueprints/BP_Player_Character.BP_Player_Character_C|GetDialogueRef (Variables|References|GetPlayerRef)) "NewEnumerator0")
          (Widget|SetVisibility (Variables|/Game/Player/Blueprints/BP_Player_Character.BP_Player_Character_C|GetDialogueRef (Variables|References|GetPlayerRef)) "Visible"))
        (:Is%20Not%20Valid
          (bind _returnvalue (UserInterface|CreateWidget "/Game/InteractableObjects/DialogueSystem/WB_DialogueBox.WB_DialogueBox_C" (Variables|References|GetPlayerControllerRef)))
          (bind _output_get (Variables|/Game/Player/Blueprints/BP_Player_Character.BP_Player_Character_C|SetDialogueRef (Variables|References|GetPlayerRef) _returnvalue))
          (Default|GetConversationPartner _output_get "NewEnumerator0" (Variables|References|GetPlayerRef))
          (Default|InitialiseDialogue _output_get "NewEnumerator0")
          (UserInterface|Viewport|AddtoViewport _output_get 0)))
      (Input|SetInputModeUIOnly (Variables|References|GetPlayerControllerRef) _output_get "DoNotLock" false)
      (Variables|/Script/Engine.PlayerController|SetbShowMouseCursor (Variables|References|GetPlayerControllerRef) true)
      (CallFunction|CreateDialogue))))

(fn ConstructionScript
  (bind _dialogue (CallFunction|AccessDialogueTable "/Game/InteractableObjects/DialogueSystem/NPC_Dialogue.NPC_Dialogue" (Variables|Dialogue|GetNPC_ID)))
  (Variables|Dialogue|SetDialogue _dialogue))

(fn CreateDialogue
  (bind (_returnedline _conversationover_) (CallFunction|GetDialogueLine "/Game/InteractableObjects/DialogueSystem/NPC_Dialogue.NPC_Dialogue" (Variables|Dialogue|GetDialogue) (Variables|Dialogue|GetConversation_ID) (Variables|Dialogue|GetLineCurrent)))
  (if _conversationover_
    (CallFunction|CloseDialogueBox)
    (Variables|Dialogue|SetLineCurrent 1)
    (Development|PrintString "Hello")
    (else
      (Rendering|Components|TextRender|SetText (Variables|/Game/InteractableObjects/DialogueSystem/WB_DialogueBox.WB_DialogueBox_C|GetBody_Text (Variables|/Game/Player/Blueprints/BP_Player_Character.BP_Player_Character_C|GetDialogueRef (Variables|References|GetPlayerRef))) _returnedline))))