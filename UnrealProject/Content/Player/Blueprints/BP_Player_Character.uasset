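; Player character Blueprint that tracks nearby interactable objects and manages interaction with them.
; InteractionRange overlaps add actors implementing BPI_InteractionInterface to InteractableObjects or remove them, sending approach and leave messages.
; Interact messages the first entry, passing the player and cached controller, while CycleInteractables moves that entry to the back.
; Key 1 prints the current list for debugging; neither Interact nor CycleInteractables is called within this Blueprint.
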(event EventBeginPlay
  (Utilities|FlowControl|Sequence
    (:then_0
      ;[1 1 1] Cast to Player Controller
      (bind _asbp_player_controller (Utilities|Casting|CastToBP_Player_Controller (Game|GetPlayerController 0)))
      (Variables|References|SetControllerRef _asbp_player_controller))))

(event OnComponentBeginOverlap(InteractionRange)
  (params (OverlappedComponent :type Primitive%20Component%20Object%20Reference) (OtherActor :type Actor%20Object%20Reference) (OtherComp :type Primitive%20Component%20Object%20Reference) (OtherBodyIndex :type Integer) (bFromSweep :type Boolean) (SweepResult :type Hit%20Result%20Structure%20%28by%20ref%29))
  ;[0.05098 0.05098 0.05098] Entering Interaction Range
  (bind _objectfound (Interaction|AddInteractable OtherActor))
  (if _objectfound
    (Class|BPIInteractionInterface|OnApproach(Message) OtherActor)
    (Development|PrintString (Utilities|GetDisplayName OtherActor))))

(event OnComponentEndOverlap(InteractionRange)
  (params (OverlappedComponent :type Primitive%20Component%20Object%20Reference) (OtherActor :type Actor%20Object%20Reference) (OtherComp :type Primitive%20Component%20Object%20Reference) (OtherBodyIndex :type Integer))
  ;[0.05098 0.05098 0.05098] Leaving Interaction Range
  (Interaction|RemoveInteractable OtherActor)
  (if true
    (Class|BPIInteractionInterface|OnLeave(Message) OtherActor)))

(event Input|KeyboardEvents|1
  (params (Key :type Key%20Structure :default "None"))
  (:Pressed
    (for _array_element (Variables|Interaction|GetInteractableObjects)
      (Development|PrintString (Utilities|GetDisplayName _array_element)))))

(fn ConstructionScript)

(fn AddInteractable
  (params (Object :type Actor%20Object%20Reference))
  (if (Utilities|DoesObjectImplementInterface Object "/Game/Player/Interfaces/BPI_InteractionInterface.BPI_InteractionInterface_C")
    (Utilities|Array|AddUnique (Variables|Interaction|GetInteractableObjects) Object)
    (return true)
    (else
      (return false))))

(fn RemoveInteractable
  (params (Object :type Actor%20Object%20Reference))
  (if (Utilities|Array|ContainsItem (Variables|Interaction|GetInteractableObjects) Object)
    (Utilities|Array|RemoveItem (Variables|Interaction|GetInteractableObjects) Object)
    (return)))

(fn CycleInteractables
  (bind _output_get (LocalVariables|SetObjectToCycle (CallFunction|GetInteractObject)))
  (Interaction|RemoveInteractable _output_get)
  (Interaction|AddInteractable _output_get)
  (return))

(fn Interact
  (bind _output_get (LocalVariables|SetObjectToInteract (CallFunction|GetInteractObject)))
  (Class|BPIInteractionInterface|OnInteract(Message) _output_get self (Variables|References|GetControllerRef)))

(fn GetInteractObject
  (return (Utilities|Array|Get(acopy) (Variables|Interaction|GetInteractableObjects))))